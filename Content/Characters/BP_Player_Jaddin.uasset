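; BP_Player_Jaddin is a player character Blueprint with logic to switch the player's view to a fixed world camera.
; GetWorldCamera searches CameraActors for the "WorldCamera" tag and passes matches to ConnectToCamera, which eases player 0's view target over with outgoing lock.
; Nothing in this file triggers it: BeginPlay is empty, and the delayed GetWorldCamera call is disconnected.
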(event `self.ReceiveBeginPlay`)

(event `GetWorldCamera`
  (bind _outactors (`GameplayStatics.GetAllActorsOfClass` "/Script/Engine.CameraActor"))
  (if (> (`KismetArrayLibrary.Array_Length` _outactors) 0)
    (for _array_element _outactors
      (if (`self.ActorHasTag` _array_element "WorldCamera")
        (`self.ConnectToCamera` _array_element)))))

(event `ConnectToCamera`
  (params (InCamera :type "CameraActor Object Reference"))
  (bind _returnvalue (`GameplayStatics.GetPlayerController` 0))
  (`/Engine/EditorBlueprintResources/StandardMacros.IsValid` _returnvalue
    (:`Is Valid`
      (`PlayerController.SetViewTargetWithBlend` _returnvalue InCamera 1.0 "VTBlend_EaseInOut" 1.0 true))))

(fn `UserConstructionScript`)