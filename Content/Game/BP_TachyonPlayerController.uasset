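; Player controller for Tachyon that sets up the player's aura, local HUD and lobby session requests.
; BeginPlay attaches an aura emitter to the controlled pawn, then, for the local controller only, waits briefly before adding the main menu and a pawn-linked player bar.
; HUD setup also shows the cursor with Game and UI input.
; Host, find and join lobby events forward to BP_TachyonGameInstance, passing the controller.
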(event `CreatePlayerAura`
  (bind _returnvalue (`self.K2_GetPawn`))
  ;[0 0 0] Create Player Aura
  (`/Engine/EditorBlueprintResources/StandardMacros.IsValid` _returnvalue
    (:`Is Valid`
      (`GameplayStatics.SpawnEmitterAttached` (`self.PlayerAura`) (`Actor.RootComponent` _returnvalue)))))

(event `self.ReceiveBeginPlay`
  ;[0 0 0] BEGIN PLAY
  (`self.CreatePlayerAura`)
  (if (`self.IsLocalController` self)
    (`self.InitHUD`)))

(event `InitHUD`
  (`KismetSystemLibrary.Delay` 0.2)
  (`self.CreateMenu` self)
  (`self.CreatePlayerBar` self)
  (`WidgetBlueprintLibrary.SetInputMode_GameAndUIEx` self null "DoNotLock" false)
  (set `self.bShowMouseCursor` true))

(event `CreateMenu`
  ;[0 0 0] Create Menu
  (bind _returnvalue (`|CreateWidget` "/Game/Widgets/MainMenu.MainMenu_C" self))
  (`/Engine/EditorBlueprintResources/StandardMacros.IsValid` _returnvalue
    (:`Is Valid`
      (`UserWidget.AddToPlayerScreen` _returnvalue 0))))

(event `CreatePlayerBar`
  ;[0 0 0] Create Player Bar
  (bind _returnvalue (`|CreateWidget` "/Game/Widgets/PlayerBar.PlayerBar_C" self))
  (`/Engine/EditorBlueprintResources/StandardMacros.IsValid` _returnvalue
    (:`Is Valid`
      (set `/Game/Widgets/PlayerBar.PawnReference` (`self.K2_GetPawn` self) _returnvalue)
      (`UserWidget.AddToPlayerScreen` _returnvalue 0))))

(event `ControllerHostLobby`
  ;[0 0 0] Host
  (bind _asbp_tachyon_game_instance (cast `/Game/Game/BP_TachyonGameInstance` (`GameplayStatics.GetGameInstance`)))
  (`/Engine/EditorBlueprintResources/StandardMacros.IsValid` _asbp_tachyon_game_instance
    (:`Is Valid`
      (`/Game/Game/BP_TachyonGameInstance.Instance_HostLobby` _asbp_tachyon_game_instance self))))

(event `ControllerFindGames`
  ;[0 0 0] Find games
  (bind _asbp_tachyon_game_instance (cast `/Game/Game/BP_TachyonGameInstance` (`GameplayStatics.GetGameInstance`)))
  (`/Engine/EditorBlueprintResources/StandardMacros.IsValid` _asbp_tachyon_game_instance
    (:`Is Valid`
      (`/Game/Game/BP_TachyonGameInstance.Instance_FindGames` _asbp_tachyon_game_instance self))))

(event `ControllerJoinLobby`
  ;[0 0 0] Join
  (bind _asbp_tachyon_game_instance (cast `/Game/Game/BP_TachyonGameInstance` (`GameplayStatics.GetGameInstance`)))
  (`/Engine/EditorBlueprintResources/StandardMacros.IsValid` _asbp_tachyon_game_instance
    (:`Is Valid`
      (`/Game/Game/BP_TachyonGameInstance.Instance_JoinLobby` _asbp_tachyon_game_instance self))))

(fn `UserConstructionScript`)