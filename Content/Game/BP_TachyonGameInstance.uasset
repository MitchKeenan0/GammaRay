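; Game instance Blueprint that handles multiplayer sessions: hosting, finding and joining games.
; Hosting creates a five-connection session, then reopens the current level as a listen server.
; Searching runs a non-LAN session query and caches results in GamesFound, from which joining always takes the first entry.
; Progress and failures are reported only through Print String messages.
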(event `Instance_HostLobby`
  (params (HostController :type "PlayerController Object Reference"))
  ;[0 0 0] Host Game
  (bind _returnvalue (`GameplayStatics.GetCurrentLevelName` true))
  (set `self.LevelName` (`KismetStringLibrary.Conv_StringToName` _returnvalue))
  (`CreateSessionCallbackProxy.CreateSession` HostController HostController 5
    (:`OnSuccess`
      (`KismetSystemLibrary.PrintString` "Opening Level..." true true (struct :`G` 0.913099 :`B` 0.254152 :`A` 1.0) 10.0)
      (`GameplayStatics.OpenLevel` (`self.LevelName`) false "listen"))
    (:`OnFailure`
      (`KismetSystemLibrary.PrintString` "Create Session Failed" true true (struct :`G` 1.0 :`B` 0.274677 :`A` 1.0) 10.0))))

(event `Instance_FindGames`
  (params (SearchingController :type "PlayerController Object Reference"))
  ;[0 0 0] Find Games
  (bind _results (`FindSessionsCallbackProxy.FindSessions` SearchingController 15000)
    (:`then`
      (`KismetSystemLibrary.PrintString` "Looking for Games..." true true (struct :`G` 1.0 :`B` 0.276372 :`A` 1.0) 10.0))
    (:`OnSuccess`
      (if (> (`KismetArrayLibrary.Array_Length` _results) 0)
        (bind _output_get (set `self.GamesFound` _results))
        (`KismetSystemLibrary.PrintString` (`KismetStringLibrary.Concat_StrStr` "Games Found: " (`KismetStringLibrary.Conv_IntToString` (`KismetArrayLibrary.Array_Length` _output_get))) true true (struct :`G` 0.991102 :`B` 0.274677 :`A` 1.0) 10.0)
        (else
          (`KismetSystemLibrary.PrintString` "No Games Found" true true (struct :`G` 1.0 :`B` 0.274677 :`A` 1.0) 10.0))))
    (:`OnFailure`
      (`KismetSystemLibrary.PrintString` "Find Sessions Failed" true true (struct :`G` 1.0 :`B` 0.274677 :`A` 1.0) 10.0))))

(event `Instance_JoinLobby`
  (params (JoiningController :type "PlayerController Object Reference"))
  (bind _gamesfound (`self.GamesFound`))
  ;[0 0 0] Join Game
  (if (> (`KismetArrayLibrary.Array_Length` _gamesfound) 0)
    (`JoinSessionCallbackProxy.JoinSession` JoiningController (`|GetArrayItem` _gamesfound)
      (:`OnSuccess`
        (`KismetSystemLibrary.PrintString` "Connecting..." true true (struct :`G` 1.0 :`B` 0.274677 :`A` 1.0) 10.0))
      (:`OnFailure`
        (`KismetSystemLibrary.PrintString` "Join Session Failed" true true (struct :`G` 1.0 :`B` 0.274677 :`A` 1.0) 10.0)))))